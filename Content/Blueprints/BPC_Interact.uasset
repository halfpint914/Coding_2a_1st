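; BPC_Interact is an interaction component for the first-person character that lets the player collect keys.
; On BeginPlay it caches the owner's camera and adds a key HUD widget to the viewport.
; Left mouse triggers a Visibility line trace, with debug drawing, from the camera out to LookDistance.
; Hitting a BP_Key sets HasKey, shows the HUD key, destroys the actor, and plays text and sound feedback.
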(event Custom|Try%20to%20Interact
  (bind _first_person_camera (Variables|Default|GetFirst%20Person%20Camera))
  (bind _returnvalue (Transformation|GetWorldLocation _first_person_camera))
  ;[0 0.1138 0.599 0.5 32] Line Trace Functionality
  (bind (_outhit _returnvalue_2) (Collision|LineTraceByChannel _returnvalue (+ _returnvalue (* (Math|Vector|GetForwardVector _first_person_camera) (Variables|Default|GetLookDistance))) "TraceTypeQuery1" false 0 "ForDuration"))
  (if _returnvalue_2
    ;[0.4271 0.3644 0.01112 0.5 28] Key Collect & Destroy
    (bind _asbp_key (Utilities|Casting|CastToBP_Key (.HitActor (Collision|BreakHitResult _outhit))))
    (Variables|Default|SetHasKey true)
    (Default|SetKeyVisible (Variables|Default|GetKeyHUD) true)
    (Actor|DestroyActor _asbp_key)
    (Development|PrintText (Utilities|Text|FormatText "Key ACQUIRED!"))
    (Audio|PlaySound2D "/Game/Audio/Keys_Jingle_A.Keys_Jingle_A" 1.0 1.0 0.0 0 0)))

(event EventBeginPlay
  ;[0 0 0 0.5 28] Camera Connection to Line Trace
  (bind _asbp_first_person_character (Utilities|Casting|CastToBP_FirstPersonCharacter (Components|GetOwner)))
  (Variables|Default|SetFirst%20Person%20Camera (Variables|/Game/FirstPerson/Blueprints/BP_FirstPersonCharacter.BP_FirstPersonCharacter_C|GetFirstPersonCamera _asbp_first_person_character))
  (bind _returnvalue (UserInterface|CreateWidget "/Game/Blueprints/WBP_KeyHUD.WBP_KeyHUD_C" (Game|GetPlayerController 0)))
  (Variables|Default|SetKeyHUD _returnvalue)
  (UserInterface|Viewport|AddtoViewport (Variables|Default|GetKeyHUD) 0))

(event Input|MouseEvents|LeftMouseButton
  (params (Key :type Key%20Structure :default "None"))
  ;[0 0.1138 0.599 0.5 32] Line Trace Functionality
  (:Pressed
    (CallFunction|TrytoInteract)))