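; BP_PhaseObject is an object that toggles between solid and phased, letting pawns pass through it while phased.
; BeginPlay creates a dynamic material instance on PhaseMesh for runtime visual changes.
; TogglePhase immediately switches the mesh's Pawn collision between Block and Ignore, while a reversible timeline animates the PhaseOpacity parameter.
; SetFocused plays or reverses a second timeline that drives HighlightStrength for a focus highlight.
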(event Custom|TogglePhase
  ;[0.2012 0.05615 0.2344 0.5] Phase Colison True or False
  (if (Variables|Default|GetIsPhased)
    (Variables|Default|SetIsPhased false)
    (Collision|SetCollisionResponsetoChannel (Variables|Default|GetPhaseMesh) "ECC_Pawn" "ECR_Block")
    (bind _phaseopacity (Timeline|TL_Phase Reverse)
      (:Update
        (Rendering|Material|SetScalarParameterValue (Variables|Default|GetPhaseMID) "PhaseOpacity" _phaseopacity :!class /Script/Engine.MaterialInstanceDynamic)))
    (else
      (Variables|Default|SetIsPhased true)
      (Collision|SetCollisionResponsetoChannel (Variables|Default|GetPhaseMesh) "ECC_Pawn" "ECR_Ignore")
      (Timeline|TL_Phase Play))))

(event Custom|SetFocused
  (params (Focused :type Boolean))
  ;[0.3177 0.2796 0.04799 0.5] Object Highlight
  (if Focused
    (bind _highlightalpha (Timeline|TL_Highlight Play)
      (:Update
        (Rendering|Material|SetScalarParameterValue (Variables|Default|GetPhaseMID) "HighlightStrength" _highlightalpha :!class /Script/Engine.MaterialInstanceDynamic)))
    (else
      (Timeline|TL_Highlight Reverse))))

(event EventBeginPlay
  ;[0.02279 0.08416 0.15 0.5] Dynamic Material
  (bind _returnvalue (Rendering|Material|CreateDynamicMaterialInstance (Variables|Default|GetPhaseMesh) 0 0 "None" :!class /Script/Engine.PrimitiveComponent))
  (Variables|Default|SetPhaseMID _returnvalue))

(fn ConstructionScript)