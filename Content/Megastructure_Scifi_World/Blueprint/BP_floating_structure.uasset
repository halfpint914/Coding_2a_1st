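; Floating megastructure prop for a sci-fi world, built from several structure mesh components that are set moving when play starts.
; On BeginPlay, each mesh or mesh pair receives a velocity-change impulse along a random unit vector at fixed strength, so the parts drift in random directions.
; Tick only runs a Delay with nothing after it, and the construction script is empty.
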(event EventBeginPlay
  (bind _returnvalue (Math|Random|RandomUnitVector))
  (bind _returnvalue_2 (Math|Float|SelectFloat -3e+01 3e+01 false))
  (bind _returnvalue_3 (* _returnvalue _returnvalue_2))
  (Physics|AddImpulse (Variables|Default|GetSM_structure_08) _returnvalue_3 "None" true)
  (Physics|AddImpulse (Variables|Default|GetSM_structure_01) _returnvalue_3 "None" true)
  (Physics|AddImpulse (Variables|Default|GetSM_structure_07) _returnvalue_3 "None" true)
  (Physics|AddImpulse (Variables|Default|GetSM_structure_06) _returnvalue_3 "None" true)
  (Physics|AddImpulse (Variables|Default|GetSM_structure_03) _returnvalue_3 "None" true)
  (Physics|AddImpulse (Variables|Default|GetSM_structure_04) _returnvalue_3 "None" true))

(event Collision|EventActorBeginOverlap
  (params (OtherActor :type Actor%20Object%20Reference)))

(event EventTick
  (params (DeltaSeconds :type Float%20%28single-precision%29))
  (Utilities|FlowControl|Delay 3.0))

(fn ConstructionScript)